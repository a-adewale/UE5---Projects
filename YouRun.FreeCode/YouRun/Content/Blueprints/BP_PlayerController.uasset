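; Player controller Blueprint that creates the player's HUD and updates its health display.
; On BeginPlay it adds a BP_HUD widget to the viewport, switches to game-only input and hides the mouse cursor.
; UpdateHealth sets the health bar, treating 100 as full, and formats the health text with a leading plus and a literal "Hi" suffix.
; A getter exposes the Sensitivity variable.
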(event `self.ReceiveBeginPlay`
  (`self.CreateHUD`)
  (`WidgetBlueprintLibrary.SetInputMode_GameOnly` self)
  (set `self.bShowMouseCursor` false))

(event `CreateHUD`
  (bind _returnvalue (`|CreateWidget` "/Game/UI/HUD/BP_HUD.BP_HUD_C"))
  (bind _output_get (set `self.HUDRef` _returnvalue))
  (`UserWidget.AddToViewport` _output_get 0))

(event `UpdateHealth`
  (params (NewHealth :type "Float (double-precision)"))
  (`ProgressBar.SetPercent` (`/Game/UI/HUD/BP_HUD.HealthBar` (`self.HUDRef`)) (/ NewHealth 100.0))
  (`TextBlock.SetText` (`/Game/UI/HUD/BP_HUD.HealthText` (`self.HUDRef`)) (`|FormatText` "+{Health} {Extra}" NewHealth "Hi")))

(fn `GetSensitivity`
  (returns (Sensitivity :type "Float (double-precision)"))
  (return (`self.Sensitivity`)))

(fn `UserConstructionScript`)