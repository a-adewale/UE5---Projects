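; First-person-style player character with movement, sensitivity-scaled look, health, and interaction with nearby pickups and physics actors.
; On BeginPlay it spawns an actor and polls by timer for the player controller to fetch sensitivity and push health.
; Overlaps track targets; Interact destroys the pickup, costing health, and impulses the InteractionActor forward.
; Zero health exits the game; left click draws a camera line trace with no further effect.
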(event `self.ReceiveBeginPlay`
  ;[0.2652 1 0.2584] Polling for references
  (bind _returnvalue (`KismetSystemLibrary.K2_SetTimer` null "Initialize" 0.01 true))
  (set `self.InitializationTimer` _returnvalue)
  (`|SpawnActorFromClass` null (`KismetMathLibrary.MakeTransform` (1880.0 -6760.0 100.0)) "Undefined" "MultiplyWithRoot" null 90.0 null))

(event `InputAxis|MoveSideWays`
  (params (AxisValue :type "Float (single-precision)"))
  ;[1 1 1] Movement and Camera
  (`self.AddMovementInput` (`self.GetActorRightVector`) AxisValue))

(event `InputAxis|MoveForward`
  (params (AxisValue :type "Float (single-precision)"))
  ;[1 1 1] Movement and Camera
  (`self.AddMovementInput` (`self.GetActorForwardVector`) AxisValue))

(event `self.ReceiveTick`
  (params (DeltaSeconds :type "Float (single-precision)")))

(event `InputAxis|LookUp`
  (params (AxisValue :type "Float (single-precision)"))
  ;[1 1 1] Movement and Camera
  (`self.AddControllerYawInput` (* AxisValue (`self.Sensitivity`))))

(event `InputAxis|LookAround`
  (params (AxisValue :type "Float (single-precision)"))
  ;[1 1 1] Movement and Camera
  (`self.AddControllerPitchInput` (* AxisValue (`self.Sensitivity`))))

(event `Key|LeftMouseButton`
  (params (Key :type "Key Structure"))
  (bind _returnvalue (`GameplayStatics.GetPlayerCameraManager` 0))
  (bind _returnvalue_2 (`self.K2_GetActorLocation` _returnvalue))
  (:`Pressed`
    (bind _outhit (`KismetSystemLibrary.LineTraceSingle` :`Start` _returnvalue_2 :`End` (+ (* (`self.GetActorForwardVector` _returnvalue) 50000.0) _returnvalue_2) :`TraceChannel` "TraceTypeQuery1" :`DrawDebugType` "Persistent"))
    (cast `` (`.HitActor` (`GameplayStatics.BreakHitResult` _outhit)))))

(event `InputAction|Interact`
  (params (Key :type "Key Structure"))
  (:`Pressed`
    (`|ExecutionSequence`
      (:`then_0`
        (`self.PickUp`))
      (:`then_1`
        (`self.NudgeBall`)))))

(event `self.ReceiveActorBeginOverlap`
  (params (OtherActor :type "Actor Object Reference"))
  (bind _asbp_pickup_actor (cast `` OtherActor)
    (:`then`
      (set `self.NearbyPickup` _asbp_pickup_actor))
    (:`CastFailed`
      (bind _asinteraction_actor (cast `/Game/Blueprints/InteractionActor` OtherActor))
      (set `self.AsInteractionActor` _asinteraction_actor))))

(event `self.ReceiveActorEndOverlap`
  (params (OtherActor :type "Actor Object Reference"))
  (bind _asbp_pickup_actor (cast `` OtherActor)
    (:`then`
      (if (== _asbp_pickup_actor (`self.NearbyPickup`))
        (set `self.NearbyPickup` null)))
    (:`CastFailed`
      (bind _asinteraction_actor (cast `/Game/Blueprints/InteractionActor` OtherActor))
      (if (== _asinteraction_actor (`self.AsInteractionActor`))
        (set `self.AsInteractionActor` null)))))

(fn `Initialize`
  (bind _asbp_player_controller (cast `/Game/Blueprints/BP_PlayerController` (`GameplayStatics.GetPlayerController` 0)))
  (`/Engine/EditorBlueprintResources/StandardMacros.IsValid` _asbp_player_controller
    (:`Is Valid`
      (set `self.PcRef` _asbp_player_controller)
      (bind _sensitivity (`/Game/Blueprints/BP_PlayerController.GetSensitivity` (`self.PcRef`)))
      (set `self.Sensitivity` _sensitivity)
      (`/Game/Blueprints/BP_PlayerController.UpdateHealth` (`self.PcRef`) (`self.Health`))
      (`KismetSystemLibrary.K2_ClearAndInvalidateTimerHandle` (`self.InitializationTimer`)))))

(fn `NudgeBall`
  (bind _asinteractionactor (`self.AsInteractionActor`)
    (:`then`
      (`PrimitiveComponent.AddImpulse` (`/Game/Blueprints/InteractionActor.StaticMesh` _asinteractionactor) (* (`self.GetActorForwardVector`) 100000.0) "None" false))
    (:`else`)))

(fn `PickUp`
  (bind _nearbypickup (`self.NearbyPickup`)
    (:`then`
      (`self.K2_DestroyActor` _nearbypickup)
      (set `self.NearbyPickup` (cast `` (`|GetArrayItem` (`self.GetOverlappingActors` null)) :!pure true))
      (`self.SetHealth` (- (`self.Health`) 40.0)))
    (:`else`)))

(fn `SetHealth`
  (params (Health :type "Float (double-precision)"))
  (bind _output_get (set `self.Health` Health))
  (if (<= _output_get 0.0)
    (`KismetSystemLibrary.ExecuteConsoleCommand` "Exit" null)
    (else
      (`/Game/Blueprints/BP_PlayerController.UpdateHealth` (`self.PcRef`) (`self.Health`)))))

(fn `UserConstructionScript`)